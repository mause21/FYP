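; BP_Door_2 is a swinging door that opens and closes when triggered while something overlaps its box collision.
; Box overlap begin and end events set a Neardoor flag.
; The Door_Open event checks that flag, then a FlipFlop alternates playing and reversing the Dooramt timeline, whose DoorRotAmt track drives the yaw of the door mesh's relative rotation.
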(event OnComponentBeginOverlap(BoxColision)
  (params (OverlappedComponent :type Primitive%20Component%20Object%20Reference) (OtherActor :type Actor%20Object%20Reference) (OtherComp :type Primitive%20Component%20Object%20Reference) (OtherBodyIndex :type Integer) (bFromSweep :type Boolean) (SweepResult :type Hit%20Result%20Structure%20%28by%20ref%29))
  (Variables|Default|SetNeardoor true))

(event OnComponentEndOverlap(BoxColision)
  (params (OverlappedComponent :type Primitive%20Component%20Object%20Reference) (OtherActor :type Actor%20Object%20Reference) (OtherComp :type Primitive%20Component%20Object%20Reference) (OtherBodyIndex :type Integer))
  (Variables|Default|SetNeardoor false))

(event Custom|Door_Open
  (if (Variables|Default|GetNeardoor)
    (Utilities|FlowControl|FlipFlop
      (:A
        (bind _doorrotamt (Timeline|Dooramt Play)
          (:Update
            (Transformation|SetRelativeRotation (Variables|Default|GetStaticMesh1) (Math|Rotator|MakeRotator 0.0 0.0 _doorrotamt) false false))))
      (:B
        (Timeline|Dooramt Reverse)))))

(fn ConstructionScript)