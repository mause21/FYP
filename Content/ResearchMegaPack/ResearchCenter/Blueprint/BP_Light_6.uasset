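; BP_Light_6 is a flickering light actor that randomly toggles the visibility of its RectLight.
; BeginPlay starts a looping half-second timer that calls FlickerEvent, where a FlipFlop alternates between two delay chains.
; One branch switches the light on, off and on again and the other switches it off, each step after a random delay of up to two seconds.
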(event Custom|FlickerEvent
  (bind _returnvalue (Math|Random|RandomFloatinRange 0.0 2.0))
  (Utilities|FlowControl|FlipFlop
    (:A
      (Utilities|FlowControl|Delay _returnvalue)
      (Rendering|SetVisibility (Variables|Default|GetRectLight) true false)
      (Utilities|FlowControl|Delay _returnvalue)
      (Rendering|SetVisibility (Variables|Default|GetRectLight) false false)
      (Utilities|FlowControl|Delay _returnvalue)
      (Rendering|SetVisibility (Variables|Default|GetRectLight) true false))
    (:B
      (Utilities|FlowControl|Delay _returnvalue)
      (Rendering|SetVisibility (Variables|Default|GetRectLight) false false))))

(event EventBeginPlay
  (bind _returnvalue (Utilities|Time|SetTimerbyEvent (delegate Custom|FlickerEvent) 0.5 true)))

(fn ConstructionScript)